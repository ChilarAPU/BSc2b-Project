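; BP_Centrifuge is an interactable centrifuge actor that opens a WBP_ProgressBar screen on overlap until HasPlayerBeaten is true.
; Box begin-overlap creates the widget, hands it a self reference and switches to game-and-UI input with a visible cursor.
; End-overlap on a separate Cube component removes all widgets, hides the cursor and restores game-only input.
; Neither overlap filters the overlapping actor, and HasPlayerBeaten is only read here.
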(event `self.Box.OnComponentBeginOverlap`
  (params (OverlappedComponent :type "PrimitiveComponent Object Reference") (OtherActor :type "Actor Object Reference") (OtherComp :type "PrimitiveComponent Object Reference") (OtherBodyIndex :type Integer) (bFromSweep :type Boolean) (SweepResult :type "HitResult Structure (by ref)"))
  (bind _returnvalue (`GameplayStatics.GetPlayerController` 0))
  (if (not (`self.HasPlayerBeaten`))
    (bind _returnvalue_2 (`|CreateWidget` "/Game/Blueprints/Widgets/WBP_ProgressBar.WBP_ProgressBar_C"))
    (`/Game/Blueprints/Widgets/WBP_ProgressBar.GetOwner` _returnvalue_2 self)
    (`UserWidget.AddToViewport` _returnvalue_2 0)
    (`WidgetBlueprintLibrary.SetInputMode_GameAndUIEx` _returnvalue null)
    (set `PlayerController.bShowMouseCursor` true _returnvalue)))

(event `self.Cube.OnComponentEndOverlap`
  (params (OverlappedComponent :type "PrimitiveComponent Object Reference") (OtherActor :type "Actor Object Reference") (OtherComp :type "PrimitiveComponent Object Reference") (OtherBodyIndex :type Integer))
  (bind _returnvalue (`GameplayStatics.GetPlayerController` 0))
  (if (not (`self.HasPlayerBeaten`))
    (`WidgetLayoutLibrary.RemoveAllWidgets`)
    (set `PlayerController.bShowMouseCursor` false _returnvalue)
    (`WidgetBlueprintLibrary.SetInputMode_GameOnly` _returnvalue)))

(fn `UserConstructionScript`)