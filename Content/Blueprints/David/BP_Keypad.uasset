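; BP_Keypad is an interactable keypad actor that opens a keypad UI when something overlaps its Box trigger, unless BHasPlayerCompleted is set.
; On overlap it switches the player to Game and UI input, ignores movement, shows the cursor and blends the view to itself.
; It then creates WBP_Keypad, passes itself through GetOwner and adds it to the viewport.
; This graph neither sets the completion flag nor restores player control.
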(event `self.Box.OnComponentBeginOverlap`
  (params (OverlappedComponent :type "PrimitiveComponent Object Reference") (OtherActor :type "Actor Object Reference") (OtherComp :type "PrimitiveComponent Object Reference") (OtherBodyIndex :type Integer) (bFromSweep :type Boolean) (SweepResult :type "HitResult Structure (by ref)"))
  (bind _returnvalue (`GameplayStatics.GetPlayerController` 0))
  (if (not (`self.BHasPlayerCompleted`))
    (`WidgetBlueprintLibrary.SetInputMode_GameAndUIEx` _returnvalue null)
    (`Controller.SetIgnoreMoveInput` _returnvalue true)
    (set `PlayerController.bShowMouseCursor` true _returnvalue)
    (`PlayerController.SetViewTargetWithBlend` _returnvalue self 1.5 "VTBlend_Linear" 0.0 false)
    (bind _returnvalue_2 (`|CreateWidget` "/Game/Blueprints/Widgets/WBP_Keypad.WBP_Keypad_C"))
    (`/Game/Blueprints/Widgets/WBP_Keypad.GetOwner` _returnvalue_2 self)
    (`UserWidget.AddToViewport` _returnvalue_2 0)))

(fn `UserConstructionScript`)